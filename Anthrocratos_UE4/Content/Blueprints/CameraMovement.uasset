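; CameraMovement is an edge-scrolling camera Blueprint that pans the actor along world Y and Z when the mouse nears a viewport border.
; Each Tick reapplies Game and UI input mode with mouse lock, then advances a looping MultiGate, so edges are checked in rotation, not together.
; A cursor within the outer tenth triggers a fixed, frame-rate-dependent step.
; The CameraUp and CameraDown variable names are opposite to their Z movement.
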(event `self.ReceiveTick`
  (params (DeltaSeconds :type "Float (single-precision)"))
  (bind _returnvalue (`GameplayStatics.GetPlayerController` 0))
  (bind (_locationx _locationy) (`PlayerController.GetMousePosition` _returnvalue))
  (bind (_x _y) (`KismetMathLibrary.BreakVector2D` (`WidgetLayoutLibrary.GetViewportSize`)))
  (bind (_x_2 _y_2) (`KismetMathLibrary.BreakVector2D` (`WidgetLayoutLibrary.GetViewportSize`)))
  (`WidgetBlueprintLibrary.SetInputMode_GameAndUIEx` _returnvalue null true)
  (`|MultiGate` false true
    (:`Out 1`
      (if (<= _locationx (* _x_2 0.1))
        (bind _output_get (set `self.CameraLeft` (`KismetMathLibrary.MakeVector` (.x (`self.K2_GetActorLocation`)) (+ (.y (`self.K2_GetActorLocation`)) -10.0) (.z (`self.K2_GetActorLocation`)))))
        (`self.K2_SetActorLocation` _output_get)))
    (:`Out 2`
      (if (>= _locationx (* _x 0.9))
        (bind _output_get_2 (set `self.CameraRight` (`KismetMathLibrary.MakeVector` (.x (`self.K2_GetActorLocation`)) (+ (.y (`self.K2_GetActorLocation`)) 10.0) (.z (`self.K2_GetActorLocation`)))))
        (`self.K2_SetActorLocation` _output_get_2)))
    (:`Out 3`
      (if (>= _locationy (* _y 0.9))
        (bind _output_get_3 (set `self.CameraUp` (`KismetMathLibrary.MakeVector` (.x (`self.K2_GetActorLocation`)) (.y (`self.K2_GetActorLocation`)) (+ (.z (`self.K2_GetActorLocation`)) -10.0))))
        (`self.K2_SetActorLocation` _output_get_3)))
    (:`Out 4`
      (if (<= _locationy (* _y_2 0.1))
        (bind _output_get_4 (set `self.CameraDown` (`KismetMathLibrary.MakeVector` (.x (`self.K2_GetActorLocation`)) (.y (`self.K2_GetActorLocation`)) (+ (.z (`self.K2_GetActorLocation`)) 10.0))))
        (`self.K2_SetActorLocation` _output_get_4)))))

(fn `UserConstructionScript`)