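; Game mode that generates a grid of hexagonal tiles when play begins.
; SpawnTiles measures a temporary HexTileBasic's mesh bounds sphere radius to derive column and row spacing, then destroys it.
; A row and column loop spawns tiles, shifting alternate columns by half a tile and storing each in the HexTiles array.
; SpawnBiomes is an empty stub.
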(event `self.ReceiveBeginPlay`
  (`self.SpawnTiles`))

(fn `SpawnBiomes`)

(fn `SpawnTiles`
  (bind _x (.x (* (`KismetMathLibrary.Conv_DoubleToVector` (`self.Xoffset`)) (`self.ColumnCounter`))))
  ;[1 1 1] Determining the unit size of tiles to then use that to determine the spawn position offset.
  (bind _returnvalue (`|SpawnActorFromClass` "/Game/Blueprints/HexTileBasic.HexTileBasic_C" (`KismetMathLibrary.MakeTransform` (0.0 0.0 0.0)) "Undefined" "OverrideRootScale"))
  (bind _output_get (set `self.HexBounds` (`.SphereRadius` (`KismetSystemLibrary.GetComponentBounds` (`/Game/Blueprints/HexTileBasic.TileMesh` _returnvalue)))))
  (`self.K2_DestroyActor` _returnvalue)
  (set `self.Xoffset` (* _output_get 1.5))
  (set `self.Yoffset` (* _output_get (`KismetMathLibrary.Sqrt` 3.0)))
  ;[1 1 1] While loop
  (while (<= (`self.RowCounter`) (`self.MaxRows`))
    ;[1 1 1] If finish row, update/reset counters
    (if (<= (`self.ColumnCounter`) (`self.MaxColumns`))
      ;[1 1 1] Checking for every "second" tile
      (if (`self.AltColumn`)
        (set `self.AltColumn` false)
        ;[1 1 1] Figuring out the next spawn position using the offset values
        (bind _output_get_2 (set `self.CurrentSpawnPos` (`KismetMathLibrary.MakeVector` _x (.x (* (`KismetMathLibrary.Conv_DoubleToVector` (`self.Yoffset`)) (`self.RowCounter`))))))
        ;[1 1 1] Spawning the tile and adding it to an array that could be used in the future
        (bind _returnvalue_2 (`|SpawnActorFromClass` "/Game/Blueprints/HexTileBasic.HexTileBasic_C" (`KismetMathLibrary.MakeTransform` _output_get_2) "Undefined" "OverrideRootScale"))
        (`KismetArrayLibrary.Array_Add` (`self.HexTiles`) _returnvalue_2)
        (else
          (set `self.AltColumn` true)
          ;[1 1 1] Every second tile gets moved up by half a tile
          (bind _output_get_3 (set `self.CurrentSpawnPos` (`KismetMathLibrary.MakeVector` _x (* (`self.Yoffset`) (.y (+ (0.5 0.5 0.5) (`self.RowCounter`)))))))
          (bind _returnvalue_3 (`|SpawnActorFromClass` "/Game/Blueprints/HexTileBasic.HexTileBasic_C" (`KismetMathLibrary.MakeTransform` _output_get_3) "Undefined" "OverrideRootScale"))
          (`KismetArrayLibrary.Array_Add` (`self.HexTiles`) _returnvalue_3)))
      (set `self.ColumnCounter` (+ (`self.ColumnCounter`) 1))
      (else
        (set `self.RowCounter` (+ (`self.RowCounter`) 1))
        (set `self.ColumnCounter` 0)
        (set `self.AltColumn` false))))
  (`KismetSystemLibrary.PrintString` "TilesGenerated"))

(fn `UserConstructionScript`)