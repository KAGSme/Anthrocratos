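; AnthroGameMode is a game mode Blueprint that tracks turn order for a turn-based game with multiple players.
; NextPlayer advances the active player index, and when it passes the player count it resets to the first player and calls EndRound.
; Debug strings print on each change, and the event graph's only NextPlayer call is not wired to any event.
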(fn `nextPlayer`
  (bind _output_get (set `self.activePlayer` (cast `EPlayerNo` (+ (`self.activePlayer`) 1))))
  (if (< _output_get (`self.players`))
    (`KismetSystemLibrary.PrintString` "next player")
    (else
      (set `self.activePlayer` "PN_0")
      (`self.EndRound`)
      (`KismetSystemLibrary.PrintString` "End Round"))))

(fn `UserConstructionScript`)