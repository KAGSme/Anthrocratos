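; Behavior tree node that copies a player's Money, Happiness and Energy into the AI's blackboard.
; On each tick it casts its owner to AI_Controller and reads the stats of the entry at index 1 in AnthroGameMode's PlayerStatObjects.
; It writes the three values as integer blackboard keys and also caches the controller and the Money value in variables.
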(event `self.ReceiveTick`
  (params (OwnerActor :type "Actor Object Reference") (DeltaSeconds :type "Float (single-precision)"))
  (bind _asai_controller (cast `/Game/Blueprints/AI/AI_Controller` OwnerActor))
  (set `self.AI_Cont` _asai_controller)
  (bind _asanthro_game_mode (cast `/Game/Blueprints/Gamemodes/AnthroGameMode` (`GameplayStatics.GetGameMode`)))
  (bind (_happiness _money _energy) (`/Game/Blueprints/Gameplay/PlayerStatsMain.GetStats` (`KismetArrayLibrary.Array_Get` (`/Game/Blueprints/Gamemodes/AnthroGameMode.PlayerStatObjects` _asanthro_game_mode) 1)))
  (`BTFunctionLibrary.SetBlackboardValueAsInt` (`self.Money_K`) _money)
  (`BTFunctionLibrary.SetBlackboardValueAsInt` (`self.Happiness_k`) _happiness)
  (`BTFunctionLibrary.SetBlackboardValueAsInt` (`self.Energy_K`) _energy)
  (set `self.NewVar_0` _money))