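; Behavior tree task that tries to place a building for the AI player in the Anthro game mode.
; When a blackboard integer is at least 30, it picks a random tile from the second player stat object and attempts to spawn building type 2 there.
; A successful spawn destroys that player stat actor, failures only print debug messages, and the task never calls Finish Execute.
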(event `self.ReceiveExecute`
  (params (OwnerActor :type "Actor Object Reference"))
  (bind _asanthro_game_mode (cast `/Game/Blueprints/Gamemodes/AnthroGameMode` (`GameplayStatics.GetGameMode`)))
  (if (>= (`BTFunctionLibrary.GetBlackboardValueAsInt` (`self.Get_M`)) 30)
    (bind _item (`KismetArrayLibrary.Array_Get` (`/Game/Blueprints/Gamemodes/AnthroGameMode.PlayerStatObjects` _asanthro_game_mode) 1))
    (bind _asai_player (cast `/Game/Blueprints/Gameplay/AI_Player` _item))
    (bind _returntiles (`/Game/Blueprints/Gameplay/AI_Player.Get Tiles` _asai_player))
    (bind _ashex_tile_basic (cast `/Game/Blueprints/Tiles/Biomes/HexTileBasic` (`KismetArrayLibrary.Array_Get` _returntiles (`KismetMathLibrary.RandomIntegerInRange` 0 (`KismetArrayLibrary.Array_Length` _returntiles)))))
    (bind _buildingtype (`/Game/Blueprints/Gameplay/PlayerStatsMain.GetBuildingType` _item 2))
    (bind _issuccessful (`/Game/Blueprints/Gameplay/PlayerStatsMain.AttemptSpawnBuilding` _item _buildingtype (`/Game/Blueprints/Tiles/Biomes/HexTileBasic.TilePosition` _ashex_tile_basic)))
    (if _issuccessful
      (`Actor.K2_DestroyActor` _item)
      (else
        (`KismetSystemLibrary.PrintString` "NotEnoughMoney/AP!")))
    (else
      (`KismetSystemLibrary.PrintString` "nae monay"))))