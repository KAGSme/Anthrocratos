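; Per-player stats actor holding Money, Food, Energy, Happiness, owned buildings and spawnable building types.
; It registers with AnthroGameMode on BeginPlay, then each round start checks Happiness against the goal for a win notification and adds funding.
; AttemptSpawnBuilding spawns the building first to read its costs, checks resources and action points, then either claims it, applying cost and tile biome, or destroys it.
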(event `/Game/Blueprints/Gameplay/iStatsAndFlows.TrackBuilding`
  (params (Building :type "/Game/Blueprints/Tiles/Buildings/Building Object Reference"))
  (`KismetArrayLibrary.Array_AddUnique` (`self.BuildingsOwned`) Building)
  (`KismetSystemLibrary.PrintString` "BuildingTracked" false))

(event `/Game/Blueprints/Gameplay/iStatsAndFlows.UntrackBuilding`
  (params (Building :type "/Game/Blueprints/Tiles/Buildings/Building Object Reference"))
  (bind _returnvalue (`KismetArrayLibrary.Array_RemoveItem` (`self.BuildingsOwned`) Building))
  (if _returnvalue
    (`KismetSystemLibrary.PrintString` "BuildingUntracked" false)))

(event `/Game/Blueprints/Gameplay/iStatsAndFlows.AddEnergy`
  (params (Energy :type Integer))
  (set `self.Energy` (+ Energy (`self.Energy`))))

(event `/Game/Blueprints/Gameplay/iStatsAndFlows.AddFood`
  (params (Food :type Integer))
  (set `self.Food` (+ Food (`self.Food`))))

(event `/Game/Blueprints/Gameplay/iStatsAndFlows.AddHappiness`
  (params (Happiness :type Integer))
  (set `self.Happiness` (+ Happiness (`self.Happiness`)))
  (`KismetSystemLibrary.PrintString` "Added Happiness" false))

(event `/Game/Blueprints/Gameplay/iStatsAndFlows.AddMoney `
  (params (MoneyAdded :type Integer))
  (set `self.Money` (+ MoneyAdded (`self.Money`))))

(event `self.ReceiveBeginPlay`
  (bind _asanthro_game_mode (cast `/Game/Blueprints/Gamemodes/AnthroGameMode` (`GameplayStatics.GetGameMode`)))
  (`/Game/Blueprints/Gamemodes/AnthroGameMode.AddPlayer` _asanthro_game_mode self)
  (add `/Game/Blueprints/Gamemodes/AnthroGameMode.StartRound` _asanthro_game_mode (delegate `StartRoundCall`)))

(event `StartRoundCall`
  (`self.CheckWinConditions`)
  (`self.AddFunding`))

(fn `AddBuildingType`
  (params (BuildingType :type "/Game/Blueprints/Tiles/Buildings/Building Class Reference") (Money :type Integer) (Food :type Integer) (Energy :type Integer))
  (bind _spawnablebuildings (`self.SpawnableBuildings`))
  (if (`KismetArrayLibrary.Array_Contains` _spawnablebuildings BuildingType)
    (`KismetSystemLibrary.PrintString` "PlayerAlreadyHasBuilding")
    (else
      (`KismetArrayLibrary.Array_AddUnique` _spawnablebuildings BuildingType))))

(fn `AddFunding`
  (bind _funding (`self.Funding`))
  (`self.AddMoney ` _funding)
  (`self.AddFood` _funding)
  (`self.AddEnergy` _funding))

(fn `AttemptSpawnBuilding`
  (params (BuildingToSpawn :type "/Game/Blueprints/Tiles/Buildings/Building Class Reference (by ref)") (HexTileRef :type "/Game/Blueprints/Tiles/Biomes/HexTileBasic Object Reference (by ref)"))
  (returns (isSuccessful :type Boolean))
  (bind _asanthro_game_mode (cast `/Game/Blueprints/Gamemodes/AnthroGameMode` (`GameplayStatics.GetGameMode`))
    (:`then`
      (bind _returnvalue (`|SpawnActorFromClass` BuildingToSpawn (`KismetMathLibrary.MakeTransform` (`/Game/Blueprints/Tiles/Biomes/HexTileBasic.TilePosition` HexTileRef) (struct) (1.0 1.0 1.0)) "Undefined" "OverrideRootScale"))
      (bind _isenough (`self.CheckResources` (`/Game/Blueprints/Tiles/Buildings/Building.money_cost` _returnvalue) (`/Game/Blueprints/Tiles/Buildings/Building.food_cost` _returnvalue) (`/Game/Blueprints/Tiles/Buildings/Building.energy_cost` _returnvalue)))
      (if _isenough
        (bind _isenoughap (`/Game/Blueprints/Gamemodes/AnthroGameMode.CheckAP` _asanthro_game_mode 1))
        (if _isenoughap
          (message `/Game/Blueprints/Gameplay/iStatsAndFlows.TrackBuilding` self _returnvalue)
          (set `/Game/Blueprints/Tiles/Buildings/Building.owner_player` self _returnvalue)
          (`/Game/Blueprints/Tiles/Buildings/Building.Cost` _returnvalue)
          (`/Game/Blueprints/Tiles/Buildings/Building.SetBiomeType` _returnvalue (`/Game/Blueprints/Tiles/Biomes/HexTileBasic.BiomeType` HexTileRef) (`PrimitiveComponent.GetMaterial` (`/Game/Blueprints/Tiles/Biomes/HexTileBasic.TileMesh` HexTileRef) 0))
          (return true)
          (else
            (`self.K2_DestroyActor` _returnvalue)
            (return false)))
        (else
          (`self.K2_DestroyActor` _returnvalue)
          (return false))))
    (:`CastFailed`
      (`KismetSystemLibrary.PrintString` "CastFailed")
      (return false))))

(fn `CheckResources`
  (params (Money :type "Integer (by ref)") (Food :type "Integer (by ref)") (Energy :type "Integer (by ref)"))
  (returns (isEnough :type Boolean))
  (if (and (>= (`self.Money`) Money) (>= (`self.Food`) Food) (>= (`self.Energy`) Energy))
    (return true)
    (else
      (return false))))

(fn `CheckWinConditions`
  (bind _asanthro_game_mode (cast `/Game/Blueprints/Gamemodes/AnthroGameMode` (`GameplayStatics.GetGameMode`)))
  (if (>= (`self.Happiness`) (`/Game/Blueprints/Gamemodes/AnthroGameMode.HappinessGoal` _asanthro_game_mode))
    (bind _asmain_controller (cast `/Game/Blueprints/Gameplay/MainController` (`GameplayStatics.GetPlayerController` 0)))
    (`/Game/Blueprints/Gameplay/MainController.AddNotification` _asmain_controller (`KismetStringLibrary.Concat_StrStr` (`|GetEnumeratorNameAsString` (`self.playerNo`)) " Wins!"))))

(fn `GetBuildingType`
  (params (`BuildingNo.` :type Integer))
  (returns (BuildingType :type "/Game/Blueprints/Tiles/Buildings/Building Class Reference"))
  (return (`KismetArrayLibrary.Array_Get` (`self.SpawnableBuildings`) `BuildingNo.`)))

(fn `GetStats`
  (returns (Happiness :type Integer) (Money :type Integer) (Energy :type Integer) (Food :type Integer))
  (return (`self.Happiness`) (`self.Money`) (`self.Energy`) (`self.Food`)))

(fn `UserConstructionScript`)