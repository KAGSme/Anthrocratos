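; AI player Blueprint that gathers the hex tiles available to it at the start of each round.
; It binds to the AnthroGameMode start-round event, then rebuilds its HexTiles array from a large sphere overlap for HexTileBasic actors, ignoring Buildings and printing each tile's name.
; GetTiles exposes that array, while GetBuildingType overrides the parent but always passes it zero instead of the requested building number.
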(event `self.ReceiveBeginPlay`
  (`parent.ReceiveBeginPlay`)
  (bind _asanthro_game_mode (cast `/Game/Blueprints/Gamemodes/AnthroGameMode` (`GameplayStatics.GetGameMode`)))
  (add `/Game/Blueprints/Gamemodes/AnthroGameMode.StartRound` _asanthro_game_mode (delegate `StartRound`)))

(event `StartRound`
  (`KismetArrayLibrary.Array_Clear` (`self.hex tiles`))
  (bind _outactors (`GameplayStatics.GetAllActorsOfClass` "/Game/Blueprints/Tiles/Buildings/Building.Building_C"))
  (bind _outactors_2 (`KismetSystemLibrary.SphereOverlapActors_NEW` (0.0 0.0 0.0) 5000.0 (`|MakeArray` "ObjectTypeQuery1" :!type "EObjectTypeQuery Enum") "/Game/Blueprints/Tiles/Biomes/HexTileBasic.HexTileBasic_C" _outactors))
  (bind _result (`/Engine/EditorBlueprintResources/StandardMacros.DecrementInt` (`KismetArrayLibrary.Array_Length` _outactors_2))
    (:`  `
      (for _index (range (+ _result 1))
        (bind _ashex_tile_basic (cast `/Game/Blueprints/Tiles/Biomes/HexTileBasic` (`KismetArrayLibrary.Array_Get` _outactors_2 _index)))
        (`KismetArrayLibrary.Array_Set` (`self.hex tiles`) _index _ashex_tile_basic true)
        (`KismetSystemLibrary.PrintString` (`KismetSystemLibrary.GetDisplayName` _ashex_tile_basic))))))

(fn `Get Tiles`
  (returns (Returntiles :type "Array of /Game/Blueprints/Tiles/Biomes/HexTileBasic Object Reference"))
  (return (`self.hex tiles`)))

(fn `GetBuildingType`
  (params (`BuildingNo.` :type Integer))
  (returns (BuildingType :type "/Game/Blueprints/Tiles/Buildings/Building Class Reference"))
  (bind _buildingtype (`parent.GetBuildingType` 0))
  (return _buildingtype))

(fn `UserConstructionScript`
  (`parent.UserConstructionScript`))