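; MainController is a controller Blueprint that sets up the game's UI and tracks the currently selected tile.
; On BeginPlay it adds the main HUD, building-upgrade and notification widgets to the viewport, hiding the latter two and caching references to all three.
; Simple getter and setter functions expose the active tile.
; AddNotification builds a SingleNotification widget from text and appends its outline element to the notification scroll box.
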(event `self.ReceiveBeginPlay`
  (bind _returnvalue (`|CreateWidget` "/Game/Blueprints/UI/HUD_Main.HUD_Main_C"))
  (set `self.HUDMainRef` _returnvalue)
  (`UserWidget.AddToViewport` _returnvalue 0)
  (bind _returnvalue_2 (`|CreateWidget` "/Game/Blueprints/UI/UpgradeBuildingUI.UpgradeBuildingUI_C"))
  (set `self.UpgradeUIRef` _returnvalue_2)
  (`UserWidget.AddToViewport` _returnvalue_2 0)
  (bind _returnvalue_3 (`|CreateWidget` "/Game/Blueprints/UI/NotificationUI.NotificationUI_C"))
  (set `self.NotificationRef` _returnvalue_3)
  (`UserWidget.AddToViewport` _returnvalue_3 0)
  (`Widget.SetVisibility` _returnvalue_3 "Hidden")
  (`Widget.SetVisibility` _returnvalue_2 "Hidden"))

(fn `AddNotification`
  (params (NotificationText :type String))
  (bind _creatednotification (`self.CreateNotification` NotificationText))
  (`PanelWidget.AddChild` (`/Game/Blueprints/UI/NotificationUI.NotificationScrollBox` (`self.NotificationRef`)) _creatednotification))

(fn `CreateNotification`
  (params (NotificationText :type String))
  (returns (CreatedNotification :type "Button Object Reference"))
  (bind _returnvalue (`|CreateWidget` "/Game/Blueprints/UI/SingleNotification.SingleNotification_C" (`GameplayStatics.GetPlayerController` 0)))
  (set `/Game/Blueprints/UI/SingleNotification.ThisNotification` NotificationText _returnvalue)
  (`TextBlock.SetText` (`/Game/Blueprints/UI/SingleNotification.NotificationText` _returnvalue) (`KismetTextLibrary.Conv_StringToText` NotificationText))
  (return (`/Game/Blueprints/UI/SingleNotification.NotificationOutline` _returnvalue)))

(fn `GetSelectedTile`
  (returns (SelectedTile :type "/Game/Blueprints/Tiles/Biomes/HexTileBasic Object Reference"))
  (return (`self.ActiveTile`)))

(fn `SetSelectedTile`
  (params (`new tile` :type "/Game/Blueprints/Tiles/Biomes/HexTileBasic Object Reference"))
  (returns (Output :type "/Game/Blueprints/Tiles/Biomes/HexTileBasic Object Reference"))
  (bind _output_get (set `self.ActiveTile` `new tile`))
  (return _output_get))

(fn `UserConstructionScript`)