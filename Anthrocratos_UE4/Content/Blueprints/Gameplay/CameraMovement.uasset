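; Player-controlled camera that pans, rotates and FOV-zooms, with optional position clamping and mouse lock.
; Keys or screen-edge cursor push a physics box with impulses, one direction per Tick via a looping MultiGate; rotation uses angular plus sideways impulses.
; Holding Confirm drags the actor directly by input axis values.
; AnthroGameMode's next-turn and end-round events play a timeline that eases the camera back to its BeginPlay transform.
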(event Custom|NextTurnCall
  (bind _startroundtransform (Variables|Default|GetStartRoundTransform))
  (bind (_location _rotation) (Math|Transform|BreakTransform _startroundtransform))
  (bind _postrack (Timeline|ResetCam PlayFromStart)
    (:Update
      (Transformation|Teleport (Math|Vector|Lerp(Vector) (Transformation|GetActorLocation) _location _postrack) (Math|Rotator|Lerp(Rotator) (Transformation|GetActorRotation) _rotation _postrack true)))))

(event EventTick
  (params (DeltaSeconds :type Float%20%28single-precision%29))
  (bind _returnvalue (Viewport|GetViewportSize))
  (bind _returnvalue_2 (Viewport|GetViewportSize))
  (bind _returnvalue_3 (Game|GetPlayerController 0))
  (bind _margin (Variables|Default|Getmargin))
  (bind (_locationx _locationy) (Game|Player|GetMousePosition _returnvalue_3))
  (bind (_x _y) (Math|Vector2D|BreakVector2D _returnvalue))
  (bind (_x_2 _y_2) (Math|Vector2D|BreakVector2D _returnvalue_2))
  (bind _returnvalue_4 (- 1.0 _margin))
  (CallFunction|MovebyCursor (Variables|Default|GetMoveOnCursor))
  (CallFunction|LockPosition (Variables|Default|GetLockMaxX) (Variables|Default|GetLockMaxY))
  (Variables|Default|SetMoveX (Math|Transform|TransformDirection (Transformation|GetActorTransform self) "1.000000, 0, 0"))
  (Variables|Default|SetMoveY (Math|Transform|TransformDirection (Transformation|GetActorTransform self) "0.000000,1.000000, 0"))
  (Variables|/Script/Engine.PlayerController|SetbShowMouseCursor _returnvalue_3 true)
  (Utilities|FlowControl|MultiGate false true -1
    (:Out%200
      ;[1 1 1] Camera Movement
      (if (or (Variables|Default|GetAHeld) (<= _locationx (* _x_2 _margin)))
        (Physics|AddImpulse (Variables|Default|GetBox) (* (* (Variables|Default|GetMoveY) -1) (Variables|Default|GetVelocity)) "None" false)))
    (:Out%201
      (if (or (Variables|Default|GetDHeld) (>= _locationx (* _x _returnvalue_4)))
        (Physics|AddImpulse (Variables|Default|GetBox) (* (Variables|Default|GetMoveY) (Variables|Default|GetVelocity)) "None" false)))
    (:Out%202
      (if (or (Variables|Default|GetSHeld) (>= _locationy (* _y _returnvalue_4)))
        (Physics|AddImpulse (Variables|Default|GetBox) (* (* (Variables|Default|GetMoveX) -1) (Variables|Default|GetVelocity)) "None" false)))
    (:Out%203
      (if (or (<= _locationy (* _y_2 _margin)) (Variables|Default|GetWHeld))
        (Physics|AddImpulse (Variables|Default|GetBox) (* (Variables|Default|GetMoveX) (Variables|Default|GetVelocity)) "None" false)))))

(event EventBeginPlay
  (Variables|Default|SetStartRoundTransform (Transformation|GetActorTransform))
  (bind _asanthro_game_mode (Utilities|Casting|CastToAnthroGameMode (Game|GetGameMode)))
  (EventDispatchers|BindEventtoNextTurn _asanthro_game_mode (delegate Custom|NextTurnCall))
  (EventDispatchers|BindEventtoEndRound _asanthro_game_mode (delegate Custom|NextTurnCall))
  (if (Variables|Default|GetLockMouse)
    (Input|SetInputModeGameandUI (Game|GetPlayerController 0) 0 true false)))

(event Input|ActionEvents|InputActionUpMovement
  (params (Key :type Key%20Structure :default "AnyKey"))
  ;[1 1 1] Keyboard Movement (Maybe this won't be needed if camera is fixed)
  (:Pressed
    (Variables|Default|SetWHeld true))
  (:Released
    (Variables|Default|SetWHeld false)))

(event Input|ActionEvents|InputActionLeftMovement
  (params (Key :type Key%20Structure :default "AnyKey"))
  ;[1 1 1] Keyboard Movement (Maybe this won't be needed if camera is fixed)
  (:Pressed
    (Variables|Default|SetAHeld true))
  (:Released
    (Variables|Default|SetAHeld false)))

(event Input|ActionEvents|InputActionDownMovement
  (params (Key :type Key%20Structure :default "AnyKey"))
  ;[1 1 1] Keyboard Movement (Maybe this won't be needed if camera is fixed)
  (:Pressed
    (Variables|Default|SetSHeld true))
  (:Released
    (Variables|Default|SetSHeld false)))

(event Input|ActionEvents|InputActionRightMovement
  (params (Key :type Key%20Structure :default "AnyKey"))
  ;[1 1 1] Keyboard Movement (Maybe this won't be needed if camera is fixed)
  (:Pressed
    (Variables|Default|SetDHeld true))
  (:Released
    (Variables|Default|SetDHeld false)))

(event Input|ActionEvents|InputActionConfirm
  (params (Key :type Key%20Structure :default "AnyKey"))
  (:Pressed
    (Variables|Default|SetMoveOnCursor true))
  (:Released
    (Variables|Default|SetMoveOnCursor false)))

(event Input|AxisEvents|InputAxisRotate
  (params (AxisValue :type Float%20%28single-precision%29))
  (CallFunction|Rotate AxisValue))

(event Input|AxisEvents|InputAxisZoom
  (params (AxisValue :type Float%20%28single-precision%29))
  (CallFunction|Zoom AxisValue))

(fn ConstructionScript)

(fn Zoom
  (params (Direction :type Float%20%28single-precision%29))
  (bind _camera (Variables|Default|GetCamera))
  (Variables|/Script/Engine.CameraComponent|SetFieldOfView _camera (Math|Float|Clamp(Float) (+ (* Direction 1e+01) (Variables|/Script/Engine.CameraComponent|GetFieldOfView _camera)) 3e+01 1.1e+02)))

(fn Rotate
  (params (Direction :type Float%20%28single-precision%29))
  (bind _box (Variables|Default|GetBox))
  (Class|PrimitiveComponent|AddAngularImpulse _box (* (Math|Vector|MakeVector 0.0 0.0 (Math|Conversions|ToFloat(Integer) (Variables|Default|GetRotationVelocity))) Direction) "None" false)
  (Physics|AddImpulse _box (* (* (Variables|Default|GetMoveY) (* -1 Direction)) (/ (Variables|Default|GetRotationVelocity) 8)) "None" false))

(fn LockPosition
  (params (X :type Float%20%28single-precision%29) (Y :type Float%20%28single-precision%29))
  (bind _returnvalue (Transformation|GetActorLocation))
  ;[1 1 1] Old
  (if (Variables|Default|GetClampPosition)
    (Transformation|SetActorLocation (Math|Vector|MakeVector (Math|Float|Clamp(Float) (.x _returnvalue) -2e+01 X) (Math|Float|Clamp(Float) (.y _returnvalue) -2e+01 Y) (.z _returnvalue)) false true)))

(fn BorderMovement)

(fn MovebyCursor
  (params (MoveOnCursor :type Boolean))
  (if MoveOnCursor
    (Transformation|SetActorLocation (+ (Transformation|GetActorLocation) (* (Variables|Default|GetMoveX) (* (Class|Actor|GetInputAxisKeyValue) (LocalVariables|GetCursormovementspeed) -1.0)) (* (Variables|Default|GetMoveY) (* (Class|Actor|GetInputAxisKeyValue) (LocalVariables|GetCursormovementspeed) -1.0))) false false)))