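; GameTileSpawner is an actor that builds a hexagonal tile map at BeginPlay.
; It measures a temporarily spawned hex tile's bounds to compute offsets, then stores a row-by-column grid of positions with alternate columns shifted half a tile.
; Basic mode fills every position with field tiles.
; Advanced mode seeds desert biomes at random indices, spreads them to neighbors via index arithmetic, and fills unused positions with field tiles.
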(event `self.ReceiveBeginPlay`
  (`self.SetSpawnTransformations`)
  (if (`self.Advanced Spawning`)
    (`self.SpawnTilesAdvanced`)
    (else
      (`self.SpawnTilesBasic`))))

(fn `SetSpawnTransformations`
  ;[1 1 1] Determining the unit size of tiles to then use that to determine the spawn position offset.
  (`self.K2_SetActorLocation` (0.0 0.0 0.0))
  (bind _returnvalue (`|SpawnActorFromClass` "/Game/Blueprints/HexTileBasic.HexTileBasic_C" (`KismetMathLibrary.MakeTransform` (0.0 0.0 0.0)) "Undefined" "OverrideRootScale"))
  (bind _output_get (set `self.HexBounds` (`.SphereRadius` (`KismetSystemLibrary.GetComponentBounds` (`/Game/Blueprints/HexTileBasic.TileMesh` _returnvalue)))))
  (`self.K2_DestroyActor` _returnvalue)
  (set `self.Xoffset` (* _output_get 1.5))
  (set `self.Yoffset` (* _output_get (`KismetMathLibrary.Sqrt` 3.0)))
  (for _index (range 1 (+ (`self.MaxRows`) 1))
    ;[1 1 1] Column For Loop
    (for _index_2 (range 1 (+ (`self.MaxColumns`) 1))
      ;[1 1 1] Checking for every "second" tile
      (if (`self.AltColumn`)
        (set `self.AltColumn` false)
        (bind _x (.x (* (`KismetMathLibrary.Conv_DoubleToVector` (`self.Xoffset`)) _index_2)))
        ;[1 1 1] Figuring out the next spawn position using the offset values
        (bind _output_get_2 (set `self.CurrentSpawnPos` (`KismetMathLibrary.MakeVector` _x (.x (* (`KismetMathLibrary.Conv_DoubleToVector` (`self.Yoffset`)) _index)))))
        ;[1 1 1] Adding the spawn position to an array of spawn transforms
        (`KismetArrayLibrary.Array_Add` (`self.SpawnTilePositions`) _output_get_2)
        (else
          (set `self.AltColumn` true)
          ;[1 1 1] Every second tile gets moved up by half a tile
          (bind _output_get_3 (set `self.CurrentSpawnPos` (`KismetMathLibrary.MakeVector` _x (* (`self.Yoffset`) (.y (+ (0.5 0.5 0.5) _index))))))
          (`KismetArrayLibrary.Array_Add` (`self.SpawnTilePositions`) _output_get_3))))
    (set `self.AltColumn` false))
  (`KismetSystemLibrary.PrintString` "TilesGenerated"))

(fn `SpawnTilesAdvanced`
  (bind _spawntilepositions (`self.SpawnTilePositions`))
  (bind _randomtilecounter (`self.RandomTileCounter`))
  (bind _usedtiles (`self.UsedTiles`))
  (bind _currenttileindex (`self.CurrentTileIndex`))
  (bind _maxcolumns (`self.MaxColumns`))
  (bind _returnvalue (`KismetArrayLibrary.Array_Length` _spawntilepositions))
  (bind _returnvalue_2 (- _currenttileindex _maxcolumns))
  (bind _returnvalue_3 (+ _currenttileindex _maxcolumns))
  (bind _returnvalue_4 (- _returnvalue_2 1))
  (bind _returnvalue_5 (- _returnvalue 1))
  (for _ (range 1 (+ (`self.MaxDesertBiomes`) 1))
    ;[1 1 1] Attempt to spawn desert tiles on unique tiles
    (bind _output_get (set `self.CurrentTileIndex` (`KismetMathLibrary.RandomInteger` _returnvalue_5)))
    (while (and (not (`KismetArrayLibrary.Array_Contains` _usedtiles _output_get)) (== _randomtilecounter 10))
      (bind _output_get_2 (set `self.CurrentTileIndex` (`KismetMathLibrary.RandomInteger` _returnvalue)))
      (set `self.RandomTileCounter` (+ _randomtilecounter 1)))
    (`KismetArrayLibrary.Array_AddUnique` _usedtiles _output_get_2)
    (`|SpawnActorFromClass` "/Game/Blueprints/DesertTile.DesertTile_C" (`KismetMathLibrary.MakeTransform` (`KismetArrayLibrary.Array_Get` _spawntilepositions _output_get)) "Undefined" "OverrideRootScale")
    ;[1 1 1] Checking if index is a valid spawn position for biome tile
    (for _index (range _returnvalue_4 (+ _returnvalue_3 1))
      (if (or (and (>= _index _returnvalue_4) (<= _index (+ _returnvalue_2 1))) (== _index _returnvalue_3) (== _index (- _currenttileindex 1)) (== _index (- _currenttileindex -1)))
        (if (and (> _index -1) (< _index _returnvalue) (not (`KismetArrayLibrary.Array_Contains` (`self.UsedTiles`) _index)))
          (`|SpawnActorFromClass` "/Game/Blueprints/DesertTile.DesertTile_C" (`KismetMathLibrary.MakeTransform` (`KismetArrayLibrary.Array_Get` (`self.SpawnTilePositions`) _index)) "Undefined" "OverrideRootScale")
          (`KismetArrayLibrary.Array_AddUnique` (`self.UsedTiles`) _index)
          (else
            (`KismetSystemLibrary.PrintString` "out of bounds"))))))
  ;[1 1 1] Once special tiles have spawned, spawn field tiles in the empty spaces
  (for _index_2 (range (+ _returnvalue_5 1))
    (if (not (`KismetArrayLibrary.Array_Contains` (`self.UsedTiles`) _index_2))
      (`|SpawnActorFromClass` "/Game/Blueprints/FieldTile.FieldTile_C" (`KismetMathLibrary.MakeTransform` (`KismetArrayLibrary.Array_Get` (`self.SpawnTilePositions`) _index_2)) "Undefined" "OverrideRootScale"))))

(fn `SpawnTilesBasic`
  (for _index (range (`KismetArrayLibrary.Array_Length` (`self.SpawnTilePositions`)))
    (`|SpawnActorFromClass` "/Game/Blueprints/FieldTile.FieldTile_C" (`KismetMathLibrary.MakeTransform` (`KismetArrayLibrary.Array_Get` (`self.SpawnTilePositions`) _index)) "Undefined" "OverrideRootScale")))

(fn `UserConstructionScript`)