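; WalkTest is a test Blueprint that adds to a Ducats counter when the W key is pressed.
; On BeginPlay it enables input, creates a HUD_Test widget, stores the reference and adds it to the viewport.
; Each W press raises Ducats by a fixed amount and prints a debug string, with no movement logic or direct update to the widget.
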(event `self.ReceiveBeginPlay`
  (`self.EnableInput` self null)
  (bind _returnvalue (`|CreateWidget` "/Game/Blueprints/HUD_Test.HUD_Test_C"))
  (bind _output_get (set `self.HUD Reference` _returnvalue))
  (`UserWidget.AddToViewport` _output_get 0))

(event `Key|W`
  (params (Key :type "Key Structure" :default "AnyKey"))
  (:`Pressed`
    (set `self.Ducats` (+ (`self.Ducats`) 2))
    (`KismetSystemLibrary.PrintString` (`self.W`))))

(fn `UserConstructionScript`)