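; PlayerStats holds a player's economy state: a Money balance and the list of buildings owned.
; Events add money and track or untrack buildings in a duplicate-free array, printing debug messages.
; RemoveMoney deducts only when the balance covers the amount, but its returned affordability check reads the balance after any deduction.
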(event `/Game/Blueprints/iStatsAndFlows.AddMoney `
  (params (MoneyAdded :type Integer))
  (set `self.Money` (+ MoneyAdded (`self.Money`))))

(event `/Game/Blueprints/iStatsAndFlows.TrackBuilding`
  (params (Building :type "Actor Object Reference"))
  (`KismetArrayLibrary.Array_AddUnique` (`self.BuildingsOwned`) Building)
  (`KismetSystemLibrary.PrintString` "BuildingTracked" false))

(event `/Game/Blueprints/iStatsAndFlows.UntrackBuilding`
  (params (Building :type "Actor Object Reference"))
  (bind _returnvalue (`KismetArrayLibrary.Array_RemoveItem` (`self.BuildingsOwned`) Building))
  (if _returnvalue
    (`KismetSystemLibrary.PrintString` "BuildingUntracked" false)))

(fn `RemoveMoney`
  (params (MoneyRemoved :type Integer))
  (returns (isSuccessful :type Boolean))
  (bind _money (`self.Money`))
  (bind _returnvalue (>= _money MoneyRemoved))
  (if _returnvalue
    (set `self.Money` (- _money MoneyRemoved)))
  (return _returnvalue))

(fn `UserConstructionScript`)