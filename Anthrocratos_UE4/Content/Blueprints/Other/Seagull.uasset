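; Seagull actor that flies in a straight line on a repeating loop.
; On BeginPlay it stores its start location and initial timer value.
; Each tick counts the timer down while setting the Box's physics linear velocity along the actor's forward vector, scaled by Speed.
; When the timer drops below zero, it resets and moves the actor back to its start location without sweeping.
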(event `self.ReceiveBeginPlay`
  (set `self.StartTimer` (`self.Timer`))
  (set `self.StartLocation` (`self.K2_GetActorLocation`)))

(event `self.ReceiveActorBeginOverlap`
  (params (OtherActor :type "Actor Object Reference")))

(event `self.ReceiveTick`
  (params (DeltaSeconds :type "Float (single-precision)"))
  (if (< (`self.Timer`) 0.0)
    (set `self.Timer` (`self.StartTimer`))
    (`self.K2_SetActorLocation` (`self.StartLocation`))
    (else
      (set `self.Timer` (- (`self.Timer`) DeltaSeconds))
      (`PrimitiveComponent.SetPhysicsLinearVelocity` (`self.Box`) (* (`self.GetActorForwardVector`) (`KismetMathLibrary.Conv_DoubleToVector` (`self.Speed`))) false "None"))))

(fn `UserConstructionScript`)