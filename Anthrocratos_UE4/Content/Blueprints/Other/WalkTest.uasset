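; WalkTest is a test Blueprint for input, a scroll-test widget and simple stat changes.
; On BeginPlay it enables input and adds a Scrolltest widget to the viewport.
; The W key prints a debug string, and the Turn_Action input raises Happiness by a fixed step.
; A Ducats increment exists but is unconnected, and the Construction Script is empty.
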(event `self.ReceiveBeginPlay`
  (`self.EnableInput` self null)
  (bind _returnvalue (`|CreateWidget` "/Game/Blueprints/UI/scrolltest.scrolltest_C"))
  (`UserWidget.AddToViewport` _returnvalue 0))

(event `Key|W`
  (params (Key :type "Key Structure" :default "AnyKey"))
  (:`Pressed`
    (`KismetSystemLibrary.PrintString` (`self.W`))))

(event `InputAction|Turn_Action`
  (params (Key :type "Key Structure" :default "AnyKey"))
  (:`Pressed`
    (set `self.Happiness` (+ (`self.Happiness`) 0.25))))

(fn `UserConstructionScript`)